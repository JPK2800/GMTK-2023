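; Game mode Blueprint that tracks gameplay time and handles progression between levels.
; Simple functions initialize, reset, add to and return a GameplayTime counter, which only changes when those functions are called.
; StartNextLevel finds the current level name in the Levels array and opens the following entry by name, doing nothing when no next entry exists.
; BeginPlay and Tick are empty.
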(fn `AddGameplayTime`
  (params (Time :type "Float (double-precision)"))
  (set `self.GameplayTime` (+ (`self.GameplayTime`) Time)))

(fn `GetGameplayTime`
  (returns (Time :type "Float (double-precision)"))
  (return (`self.GameplayTime`)))

(fn `InitGameplayTime`
  (set `self.GameplayTime` 0.0))

(fn `ResetGameplayTime`
  (set `self.GameplayTime` 0.0))

(fn `StartNextLevel`
  (locals (LevelIndex :type Integer :default 0))
  (bind _returnvalue (+ (`local.LevelIndex`) 1))
  (bind _returnvalue_2 (`GameplayStatics.GetCurrentLevelName` true))
  (set `local.LevelIndex` (`KismetArrayLibrary.Array_Find` (`self.Levels`) _returnvalue_2))
  (if (`KismetArrayLibrary.Array_IsValidIndex` (`self.Levels`) _returnvalue)
    (`GameplayStatics.OpenLevel` (`KismetStringLibrary.Conv_StringToName` (`|GetArrayItem` (`self.Levels`) _returnvalue)))))

(fn `UserConstructionScript`)