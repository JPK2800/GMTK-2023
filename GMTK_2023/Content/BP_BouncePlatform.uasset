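; BP_BouncePlatform is a platform that launches BP_Protag away when it touches one of four side triggers.
; Top, bottom, left and right overlaps overwrite the protagonist capsule's physics velocity along an up or forward axis derived from the platform's relative rotation with a 180-degree flip.
; Each bounce also plays the platform's bounce animation.
; The LockPlatform override calls its parent, then swaps between yellow and red materials to show the locked state.
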(event `self.TopCollision.OnComponentBeginOverlap`
  (params (OverlappedComponent :type "PrimitiveComponent Object Reference") (OtherActor :type "Actor Object Reference") (OtherComp :type "PrimitiveComponent Object Reference") (OtherBodyIndex :type Integer) (bFromSweep :type Boolean) (SweepResult :type "HitResult Structure (by ref)"))
  (bind _asbp_protag (cast `/Game/BP_Protag` OtherActor))
  (`PrimitiveComponent.SetPhysicsLinearVelocity` (`/Game/BP_Protag.Capsule` _asbp_protag) (* (`KismetMathLibrary.GetUpVector` (`KismetMathLibrary.ComposeRotators` (`SceneComponent.RelativeRotation` (`self.Platform`)) (struct :`Yaw` 180.0))) 5000.0) false "None")
  (`SkeletalMeshComponent.PlayAnimation` (`self.BouncePlatform`) "/Game/platform_rectangleBounce_Anim_Root_bounce.platform_rectangleBounce_Anim_Root_bounce" false))

(event `self.BottomCollision.OnComponentBeginOverlap`
  (params (OverlappedComponent :type "PrimitiveComponent Object Reference") (OtherActor :type "Actor Object Reference") (OtherComp :type "PrimitiveComponent Object Reference") (OtherBodyIndex :type Integer) (bFromSweep :type Boolean) (SweepResult :type "HitResult Structure (by ref)"))
  (bind _asbp_protag (cast `/Game/BP_Protag` OtherActor))
  (`PrimitiveComponent.SetPhysicsLinearVelocity` (`/Game/BP_Protag.Capsule` _asbp_protag) (* (`KismetMathLibrary.GetUpVector` (`KismetMathLibrary.ComposeRotators` (`SceneComponent.RelativeRotation` (`self.Platform`)) (struct :`Yaw` 180.0))) -5000.0) false "None")
  (`SkeletalMeshComponent.PlayAnimation` (`self.BouncePlatform`) "/Game/platform_rectangleBounce_Anim_Root_bounce.platform_rectangleBounce_Anim_Root_bounce" false))

(event `self.LeftCollision.OnComponentBeginOverlap`
  (params (OverlappedComponent :type "PrimitiveComponent Object Reference") (OtherActor :type "Actor Object Reference") (OtherComp :type "PrimitiveComponent Object Reference") (OtherBodyIndex :type Integer) (bFromSweep :type Boolean) (SweepResult :type "HitResult Structure (by ref)"))
  (bind _asbp_protag (cast `/Game/BP_Protag` OtherActor))
  (`PrimitiveComponent.SetPhysicsLinearVelocity` (`/Game/BP_Protag.Capsule` _asbp_protag) (* (`KismetMathLibrary.GetForwardVector` (`KismetMathLibrary.ComposeRotators` (`SceneComponent.RelativeRotation` (`self.Platform`)) (struct :`Yaw` 180.0))) -5000.0) false "None")
  (`SkeletalMeshComponent.PlayAnimation` (`self.BouncePlatform`) "/Game/platform_rectangleBounce_Anim_Root_bounce.platform_rectangleBounce_Anim_Root_bounce" false))

(event `self.RightCollision.OnComponentBeginOverlap`
  (params (OverlappedComponent :type "PrimitiveComponent Object Reference") (OtherActor :type "Actor Object Reference") (OtherComp :type "PrimitiveComponent Object Reference") (OtherBodyIndex :type Integer) (bFromSweep :type Boolean) (SweepResult :type "HitResult Structure (by ref)"))
  (bind _asbp_protag (cast `/Game/BP_Protag` OtherActor))
  (`PrimitiveComponent.SetPhysicsLinearVelocity` (`/Game/BP_Protag.Capsule` _asbp_protag) (* (`KismetMathLibrary.GetForwardVector` (`KismetMathLibrary.ComposeRotators` (`SceneComponent.RelativeRotation` (`self.Platform`)) (struct :`Yaw` 180.0))) 5000.0) false "None")
  (`SkeletalMeshComponent.PlayAnimation` (`self.BouncePlatform`) "/Game/platform_rectangleBounce_Anim_Root_bounce.platform_rectangleBounce_Anim_Root_bounce" false))

(fn `LockPlatform`
  (bind _bounceplatform (`self.BouncePlatform`))
  (`parent.LockPlatform`)
  (if (`self.Locked`)
    (`PrimitiveComponent.SetMaterial` _bounceplatform 0 "/Game/MI_YellowPlatform.MI_YellowPlatform")
    (else
      (`PrimitiveComponent.SetMaterial` _bounceplatform 0 "/Game/MI_RedPlatform.MI_RedPlatform"))))

(fn `UserConstructionScript`
  (`parent.UserConstructionScript`))