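; Player controller for a level-based platform puzzle: the player hops between linked BP_Platform pawns to rotate, move and lock them.
; Input feeds the possessed platform, while possession changes set up its camera and toggle current, left and right neighbor widgets.
; Reset restores BP_Protag actors with physics and starts the level timer on first press.
; It also manages tip and victory widgets, reports time to BP_GameMode and requests the next level.
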(event `self.ReceiveTick`
  (params (DeltaSeconds :type "Float (single-precision)"))
  (`self.AddLevelTime` DeltaSeconds))

(event `InputAxis|RotateLeft`
  (params (AxisValue :type "Float (single-precision)"))
  (bind _platform (`self.Platform`))
  (`/Engine/EditorBlueprintResources/StandardMacros.IsValid` _platform
    (:`Is Valid`
      (set `/Game/BP_Platform.RotateLeftValue` AxisValue _platform))))

(event `InputAxis|RotateRight`
  (params (AxisValue :type "Float (single-precision)"))
  (bind _platform (`self.Platform`))
  (`/Engine/EditorBlueprintResources/StandardMacros.IsValid` _platform
    (:`Is Valid`
      (set `/Game/BP_Platform.RotateRightValue` AxisValue _platform))))

(event `InputAxis|MoveHorizontal`
  (params (AxisValue :type "Float (single-precision)"))
  (bind _platform (`self.Platform`))
  (`/Engine/EditorBlueprintResources/StandardMacros.IsValid` _platform
    (:`Is Valid`
      (set `/Game/BP_Platform.MoveHorizontalValue` AxisValue _platform))))

(event `InputAxis|MoveVertical`
  (params (AxisValue :type "Float (single-precision)"))
  (bind _platform (`self.Platform`))
  (`/Engine/EditorBlueprintResources/StandardMacros.IsValid` _platform
    (:`Is Valid`
      (set `/Game/BP_Platform.MoveVerticalValue` AxisValue _platform))))

(event `InputAction|PossessRight`
  (params (Key :type "Key Structure"))
  (bind _platform (`self.Platform`))
  (bind _rightplatform (`/Game/BP_Platform.RightPlatform` _platform))
  (:`Pressed`
    (`/Engine/EditorBlueprintResources/StandardMacros.IsValid` _platform
      (:`Is Valid`
        (`/Engine/EditorBlueprintResources/StandardMacros.IsValid` _rightplatform
          (:`Is Valid`
            (`self.Possess` _rightplatform)))))))

(event `InputAction|PossessLeft`
  (params (Key :type "Key Structure"))
  (bind _platform (`self.Platform`))
  (bind _leftplatform (`/Game/BP_Platform.LeftPlatform` _platform))
  (:`Pressed`
    (`/Engine/EditorBlueprintResources/StandardMacros.IsValid` _platform
      (:`Is Valid`
        (`/Engine/EditorBlueprintResources/StandardMacros.IsValid` _leftplatform
          (:`Is Valid`
            (`self.Possess` _leftplatform)))))))

(event `self.ReceivePossess`
  (params (PossessedPawn :type "Pawn Object Reference"))
  (bind _asbp_platform (cast `/Game/BP_Platform` PossessedPawn))
  (bind _output_get (set `self.Platform` _asbp_platform))
  (`/Game/BP_Platform.OnPossessInitCamera` _output_get)
  (`KismetSystemLibrary.Delay` 0.1)
  (`/Game/BP_Platform.DisplayWidget` _asbp_platform false false true true)
  (`|ExecutionSequence`
    (:`then_0`
      (bind _leftplatform (`/Game/BP_Platform.LeftPlatform` _output_get))
      (`/Engine/EditorBlueprintResources/StandardMacros.IsValid` _leftplatform
        (:`Is Valid`
          (`/Game/BP_Platform.DisplayWidget` _leftplatform true false true false))))
    (:`then_1`
      (bind _rightplatform (`/Game/BP_Platform.RightPlatform` _output_get))
      (`/Engine/EditorBlueprintResources/StandardMacros.IsValid` _rightplatform
        (:`Is Valid`
          (`/Game/BP_Platform.DisplayWidget` _rightplatform false true true false))))))

(event `self.ReceiveUnPossess`
  (params (UnpossessedPawn :type "Pawn Object Reference"))
  (bind _asbp_platform (cast `/Game/BP_Platform` UnpossessedPawn))
  (`/Game/BP_Platform.UnpossessResetValues` _asbp_platform)
  (`|ExecutionSequence`
    (:`then_0`
      (bind _leftplatform (`/Game/BP_Platform.LeftPlatform` _asbp_platform))
      (`/Engine/EditorBlueprintResources/StandardMacros.IsValid` _leftplatform
        (:`Is Valid`
          (`/Game/BP_Platform.DisplayWidget` _leftplatform false false false false))))
    (:`then_1`
      (bind _rightplatform (`/Game/BP_Platform.RightPlatform` _asbp_platform))
      (`/Engine/EditorBlueprintResources/StandardMacros.IsValid` _rightplatform
        (:`Is Valid`
          (`/Game/BP_Platform.DisplayWidget` _rightplatform false false false false))))))

(event `InputAction|Reset`
  (params (Key :type "Key Structure"))
  (:`Pressed`
    (if (not (`self.LevelComplete`))
      (bind _outactors (`GameplayStatics.GetAllActorsOfClass` "/Game/BP_Protag.BP_Protag_C"))
      (for _array_element _outactors
        (`/Game/BP_Protag.ResetPosition` _array_element)
        (`/Game/BP_Protag.EnablePhysics` _array_element))
      (`self.RemoveResetTip`)
      (`self.RemoveStartTip`)
      (`self.StartLevelTimer`))))

(event `InputAction|LockPos`
  (params (Key :type "Key Structure"))
  (bind _platform (`self.Platform`))
  (:`Pressed`
    (`/Engine/EditorBlueprintResources/StandardMacros.IsValid` _platform
      (:`Is Valid`
        (`/Game/BP_Platform.LockPlatform` _platform)))))

(event `InputAction|Start`
  (params (Key :type "Key Structure"))
  (:`Pressed`
    (if (`self.LevelComplete`)
      (bind _asbp_game_mode (cast `/Game/BP_GameMode` (`GameplayStatics.GetGameMode`)))
      (`/Game/BP_GameMode.StartNextLevel` _asbp_game_mode))))

(fn `AddLevelTime`
  (params (DeltaTime :type "Float (double-precision)"))
  (set `self.LevelTimerSeconds` (+ (`self.LevelTimerSeconds`) DeltaTime)))

(fn `AddResetTip`
  (if (not (`self.LevelComplete`))
    (bind _returnvalue (`|CreateWidget` "/Game/WBP_ResetTip.WBP_ResetTip_C"))
    (`UserWidget.AddToViewport` _returnvalue 0)
    (set `self.ResetTip` _returnvalue)))

(fn `AddStartTip`
  (bind _returnvalue (`|CreateWidget` "/Game/WBP_Start_StartButton.WBP_Start_StartButton_C"))
  (`UserWidget.AddToViewport` _returnvalue 0)
  (set `self.StartTip` _returnvalue))

(fn `AddVictoryLevelWidget`
  (bind _asbp_game_mode (cast `/Game/BP_GameMode` (`GameplayStatics.GetGameMode`)))
  (bind _returnvalue (`|CreateWidget` "/Game/WBP_Victory.WBP_Victory_C" null (`KismetTextLibrary.Conv_DoubleToText` (`self.LevelTimerSeconds`) "HalfToEven") (`KismetTextLibrary.Conv_DoubleToText` (`/Game/BP_GameMode.GetGameplayTime` _asbp_game_mode) "HalfToEven")))
  (`UserWidget.AddToViewport` _returnvalue 0)
  (set `self.VictoryWidget` _returnvalue)
  (set `self.LevelComplete` true))

(fn `EndLevelTime`
  (set `self.TimerEnded` true)
  (bind _asbp_game_mode (cast `/Game/BP_GameMode` (`GameplayStatics.GetGameMode`)))
  (`/Game/BP_GameMode.AddGameplayTime` _asbp_game_mode (`self.LevelTimerSeconds`)))

(fn `RemoveResetTip`
  (bind _resettip (`self.ResetTip`))
  (`/Engine/EditorBlueprintResources/StandardMacros.IsValid` _resettip
    (:`Is Valid`
      (`Widget.RemoveFromParent` _resettip)
      (set `self.ResetTip` null))))

(fn `RemoveStartTip`
  (bind _starttip (`self.StartTip`))
  (`/Engine/EditorBlueprintResources/StandardMacros.IsValid` _starttip
    (:`Is Valid`
      (`Widget.RemoveFromParent` _starttip)
      (set `self.StartTip` null))))

(fn `StartLevelTimer`
  (if (not (`self.TimerStarted`))
    (set `self.LevelTimerSeconds` 0.0)
    (set `self.TimerStarted` true)))

(fn `UserConstructionScript`)