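; BP_Protag is the protagonist actor, a physics-simulated capsule with a skeletal mesh that can reset to its spawn location.
; Each Tick it detects falling too low or straying far from the player controller, then auto-resets in Lvl_Menu or toggles a reset tip through BP_PlayerController elsewhere.
; Resetting zeroes linear and angular velocity and briefly hides the mesh on a timer.
; Helper functions show a start tip and switch off gravity.
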(event `self.ReceiveBeginPlay`
  (set `self.InitialLoc` (`self.K2_GetActorLocation`))
  (`self.EnablePhysics`))

(event `self.ReceiveTick`
  (params (DeltaSeconds :type "Float (single-precision)"))
  (`self.ResetTipIfTooFar`))

(fn `DisablePhysics`
  (`PrimitiveComponent.SetEnableGravity` (`self.Capsule`) false))

(fn `DisableVisibilityOnReset`
  (bind _returnvalue (`KismetSystemLibrary.K2_SetTimer` null "ReenableVisiblityOnReset" 0.25))
  (set `self.VisResetTimer` _returnvalue)
  (`SceneComponent.SetVisibility` (`self.SkeletalMesh`) false false))

(fn `EnablePhysics`
  (`PrimitiveComponent.SetSimulatePhysics` (`self.Capsule`) true)
  (`self.ResetPosition`))

(fn `InitializeTip`
  (bind _asbp_player_controller (cast `/Game/BP_PlayerController` (`GameplayStatics.GetPlayerController` 0)))
  (`/Game/BP_PlayerController.AddStartTip` _asbp_player_controller))

(fn `ReenableVisiblityOnReset`
  (`SceneComponent.SetVisibility` (`self.SkeletalMesh`) true false))

(fn `ResetPosition`
  (bind _capsule (`self.Capsule`))
  (`self.DisableVisibilityOnReset`)
  (`SceneComponent.K2_SetRelativeLocationAndRotation` :`self` _capsule :`NewLocation` (`self.InitialLoc`))
  (`PrimitiveComponent.SetPhysicsLinearVelocity` _capsule (0.0 0.0 0.0) false "None")
  (`PrimitiveComponent.SetPhysicsAngularVelocityInDegrees` _capsule (0.0 0.0 0.0) false "None")
  (set `self.ShowingTip` false))

(fn `ResetTipIfTooFar`
  (bind _capsule (`self.Capsule`))
  (bind (_returnvalue_x _returnvalue_y _returnvalue_z) (`KismetMathLibrary.BreakVector` (`SceneComponent.K2_GetComponentLocation` _capsule)))
  (if (or (< _returnvalue_z -2000.0) (> (`KismetMathLibrary.Vector_Distance` (`self.K2_GetActorLocation` (`GameplayStatics.GetPlayerController` 0)) (`SceneComponent.K2_GetComponentLocation` _capsule)) 20000.0))
    (bind _returnvalue (`GameplayStatics.GetCurrentLevelName` true))
    (if (`KismetStringLibrary.EqualEqual_StrStr` _returnvalue "Lvl_Menu")
      (`self.ResetPosition`)
      (elif (not (`self.ShowingTip`))
        (bind _asbp_player_controller (cast `/Game/BP_PlayerController` (`GameplayStatics.GetPlayerController` 0)))
        (`/Game/BP_PlayerController.AddResetTip` _asbp_player_controller)
        (set `self.ShowingTip` true)))
    (elif (`self.ShowingTip`)
      (bind _asbp_player_controller_2 (cast `/Game/BP_PlayerController` (`GameplayStatics.GetPlayerController` 0)))
      (`/Game/BP_PlayerController.RemoveResetTip` _asbp_player_controller_2)
      (set `self.ShowingTip` false))))

(fn `UserConstructionScript`)