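; Possessable puzzle-style platform that the player slides horizontally and vertically and rotates left or right.
; Tick turns stored input values into motion through opposing interpolations that spring back toward rest, resetting the transform when uncontrolled.
; Locking freezes the platform in place and swaps its material.
; On possession the camera starts at the player's view and glides onto its target, while a helper drives the button-prompt widget.
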(event `self.ReceiveTick`
  (params (DeltaSeconds :type "Float (single-precision)"))
  (`self.RotateLeftStep` DeltaSeconds)
  (`self.RotateRightStep` DeltaSeconds)
  (`self.MoveStep` DeltaSeconds)
  (`self.OnPossessInterpCameraStep` DeltaSeconds)
  (`self.UnpossessedResetInterp` DeltaSeconds))

(fn `DisplayWidget`
  (params (L :type Boolean) (R :type Boolean) (Visible :type Boolean) (Current :type Boolean))
  (bind _widget (`self.Widget`))
  (`SceneComponent.SetVisibility` _widget Visible false)
  (if Visible
    (bind _aswbp_button_widget (cast `/Game/UI/WBP_ButtonWidget` (`WidgetComponent.GetWidget` _widget)))
    (`/Game/UI/WBP_ButtonWidget.UpdateVisibility` _aswbp_button_widget Current L R (not Visible))))

(fn `LockPlatform`
  (bind _platform (`self.Platform`))
  (if (`self.Locked`)
    (set `self.Locked` false)
    (`PrimitiveComponent.SetMaterial` _platform 0 "/Game/Platforms/MI_RedPlatform.MI_RedPlatform")
    (else
      (set `self.Locked` true)
      (`PrimitiveComponent.SetMaterial` _platform 0 "/Game/Platforms/MI_YellowPlatform.MI_YellowPlatform"))))

(fn `MoveStep`
  (params (DeltaTime :type "Float (double-precision)"))
  (bind _platform (`self.Platform`))
  (bind _returnvalue (`KismetMathLibrary.MakeVector` (`self.MoveHorizontalValue`) 0.0 (`self.MoveVerticalValue`)))
  (bind _relativelocation (`SceneComponent.RelativeLocation` _platform))
  (bind _returnvalue_2 (`KismetMathLibrary.VSize` (`KismetMathLibrary.Normal` _returnvalue)))
  (if (not (`self.Locked`))
    (`|ExecutionSequence`
      (:`then_0`
        (if (> _returnvalue_2 0.0)
          (`SceneComponent.K2_SetRelativeLocation` _platform (`KismetMathLibrary.VInterpTo` _relativelocation (* _returnvalue 9000.0) DeltaTime _returnvalue_2) true false)))
      (:`then_1`
        (`SceneComponent.K2_SetRelativeLocation` _platform (`KismetMathLibrary.VInterpTo` _relativelocation (0.0 0.0 0.0) DeltaTime (- (* (- 5.0 _returnvalue_2) 2.0) 2.0)) true false)))))

(fn `OnPossessInitCamera`
  (`SceneComponent.K2_SetWorldLocation` (`self.Camera`) (`PlayerCameraManager.GetCameraLocation` (`GameplayStatics.GetPlayerCameraManager` 0)) false false)
  (set `self.CamSnapped` false))

(fn `OnPossessInterpCameraStep`
  (params (DeltaTime :type "Float (double-precision)"))
  (bind _camera (`self.Camera`))
  (if (> (`KismetMathLibrary.VSize` (`SceneComponent.RelativeLocation` (`self.Camera`))) 5.0)
    (`SceneComponent.K2_SetWorldLocation` _camera (`KismetMathLibrary.VInterpTo` (`SceneComponent.K2_GetComponentLocation` _camera) (`SceneComponent.K2_GetComponentLocation` (`self.CamTarg`)) DeltaTime 25.0) false false)
    (elif (not (`self.CamSnapped`))
      (`SceneComponent.K2_SetRelativeLocation` (`self.Camera`) (0.0 0.0 0.0) false false)
      (set `self.CamSnapped` true))))

(fn `RotateLeftStep`
  (params (DeltaTime :type "Float (double-precision)"))
  (bind _platform (`self.Platform`))
  (bind _rotateleftvalue (`self.RotateLeftValue`))
  (bind _platform_2 (`self.Platform`))
  (if (`self.Locked`)
    _
    (elif (> (`KismetMathLibrary.Abs` _rotateleftvalue) 0.2)
      (`SceneComponent.K2_SetRelativeRotation` _platform_2 (`KismetMathLibrary.RInterpTo` (`SceneComponent.RelativeRotation` _platform_2) (struct :`Pitch` 90.0) DeltaTime (* _rotateleftvalue 4.0)) false false)
      (else
        (`SceneComponent.K2_SetRelativeRotation` _platform (`KismetMathLibrary.RInterpTo` (`SceneComponent.RelativeRotation` _platform) (struct) DeltaTime 2.0) false false)))))

(fn `RotateRightStep`
  (params (DeltaTime :type "Float (double-precision)"))
  (bind _platform (`self.Platform`))
  (bind _platform_2 (`self.Platform`))
  (bind _returnvalue (`KismetMathLibrary.Abs` (`self.RotateRightValue`)))
  (if (`self.Locked`)
    _
    (elif (> _returnvalue 0.2)
      (`SceneComponent.K2_SetRelativeRotation` _platform_2 (`KismetMathLibrary.RInterpTo` (`SceneComponent.RelativeRotation` _platform_2) (struct :`Pitch` -90.0) DeltaTime (* _returnvalue 4.0)) false false)
      (else
        (`SceneComponent.K2_SetRelativeRotation` _platform (`KismetMathLibrary.RInterpTo` (`SceneComponent.RelativeRotation` _platform) (struct) DeltaTime 2.0) false false)))))

(fn `UnpossessedResetInterp`
  (params (DeltaTime :type "Float (double-precision)"))
  (bind _platform (`self.Platform`))
  (if (and (not (`self.Locked`)) (not (`self.IsControlled`)))
    (`SceneComponent.K2_SetRelativeTransform` _platform (`KismetMathLibrary.TInterpTo` (`SceneComponent.GetRelativeTransform` _platform) (`KismetMathLibrary.MakeTransform` (0.0 0.0 0.0)) DeltaTime 5.0) false false)))

(fn `UnpossessResetValues`
  (set `self.RotateLeftValue` 0.0)
  (set `self.RotateRightValue` 0.0)
  (set `self.MoveHorizontalValue` 0.0)
  (set `self.MoveVerticalValue` 0.0))

(fn `UserConstructionScript`)