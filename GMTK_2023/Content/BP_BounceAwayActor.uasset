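; BP_BounceAwayActor is a bumper that knocks the player character, BP_Protag, away from itself on contact.
; When its Sphere component begins overlapping the player, it computes the direction from the actor's location to the overlapping component.
; It then replaces the physics linear velocity of the player's Capsule with that normalized direction scaled by Power, rather than adding to the existing velocity.
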(event `self.Sphere.OnComponentBeginOverlap`
  (params (OverlappedComponent :type "PrimitiveComponent Object Reference") (OtherActor :type "Actor Object Reference") (OtherComp :type "PrimitiveComponent Object Reference") (OtherBodyIndex :type Integer) (bFromSweep :type Boolean) (SweepResult :type "HitResult Structure (by ref)"))
  (bind (_returnvalue_x _returnvalue_y _returnvalue_z) (`KismetMathLibrary.BreakVector` (`KismetMathLibrary.GetForwardVector` (`KismetMathLibrary.FindLookAtRotation` (`self.K2_GetActorLocation`) (`SceneComponent.K2_GetComponentLocation` OtherComp)))))
  (bind _asbp_protag (cast `/Game/BP_Protag` OtherActor))
  (`PrimitiveComponent.SetPhysicsLinearVelocity` (`/Game/BP_Protag.Capsule` _asbp_protag) (* (`KismetMathLibrary.Normal` (`KismetMathLibrary.MakeVector` _returnvalue_x _returnvalue_y _returnvalue_z)) (`self.Power`)) false "None"))

(fn `UserConstructionScript`)